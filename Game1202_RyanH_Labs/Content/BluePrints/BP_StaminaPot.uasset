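; BP_StaminaPot is a pickup that restores stamina to the player.
; On any actor overlap it runs the parent logic, then casts player character 0 to BP_Player without checking which actor overlapped.
; It adds a fixed amount to Stamina with no clamp here, then calls ItemCollected after a short delay.
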(event EventBeginPlay
  (|CallParentFunction) ; This node is disabled and will not be called.\nDrag off pins to build functionality.
)

(event Collision|EventActorBeginOverlap
  (params (OtherActor :type Actor%20Object%20Reference))
  (|CallParentFunction OtherActor)
  (bind _asbp_player (Utilities|Casting|CastToBP_Player (Game|GetPlayerCharacter 0)))
  (Variables|Default|SetAs%20BP%20Player _asbp_player)
  (Variables|/Game/BluePrints/BP_Player.BP_Player_C|SetStamina (Variables|Default|GetAs%20BP%20Player) (+ (Variables|/Game/BluePrints/BP_Player.BP_Player_C|GetStamina (Variables|Default|GetAs%20BP%20Player)) 25.0))
  (Utilities|FlowControl|Delay 0.2)
  (CallFunction|ItemCollected))

(fn ConstructionScript
  (|CallParentFunction))